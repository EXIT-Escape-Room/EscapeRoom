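; Clickable payphone for a riddle that opens a numpad widget when the player has a coin and the required item active.
; The numpad receives the correct number as its password, and the first-person character's rotation is disabled.
; Without a coin, a temporary dialog says money is needed, with a stored widget reference preventing duplicates.
; Cursor hover toggles custom depth rendering on the payphone.
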(event OnClicked(payphone)
  (params (TouchedComponent :type Primitive%20Component%20Object%20Reference) (ButtonPressed :type Key%20Structure :default "None"))
  (bind _asfirst_person_character (Utilities|Casting|CastToFirstPersonCharacter (Game|GetPlayerCharacter 0)))
  (if (Variables|/Game/FirstPersonBP/Blueprints/FirstPersonCharacter.FirstPersonCharacter_C|GetHasCoin _asfirst_person_character)
    (bind _activeitem (Utilities|GetActiveItem))
    (if (Utilities|Enum|Equal(Enum) _activeitem (Variables|Default|GetActiveItem))
      (Utilities|IsValid "/Game/PayphoneRiddle/WB_PhoneNumpad.WB_PhoneNumpad"
        (:Is%20Valid
          (bind _returnvalue (UserInterface|CreateWidget "/Game/PayphoneRiddle/WB_PhoneNumpad.WB_PhoneNumpad_C" 0 (Variables|Default|GetCorrectNumber) 0))
          (bind _output_get (Variables|Default|SetNumpadWidget _returnvalue))
          (UserInterface|Viewport|AddtoViewport _output_get 0)
          (bind _asfirst_person_character_2 (Utilities|Casting|CastToFirstPersonCharacter (Game|GetPlayerCharacter 0)))
          (Variables|/Game/FirstPersonBP/Blueprints/FirstPersonCharacter.FirstPersonCharacter_C|SetCanRotate _asfirst_person_character_2 false))))
    (else
      (Variables|Default|GetIsValid
        (:then)
        (:else
          (bind _returnvalue_2 (UserInterface|CreateWidget "/Game/FirstPersonBP/Feedback/WB_CharacterDialog.WB_CharacterDialog_C" 0 "I need money to use this phone."))
          (Variables|Default|SetIsValid _returnvalue_2)
          (UserInterface|Viewport|AddtoViewport _returnvalue_2 0)
          (Utilities|FlowControl|Delay 3.0)
          (Widget|RemovefromParent _returnvalue_2)
          (Variables|Default|SetIsValid 0))))))

(event OnBeginCursorOver(payphone)
  (params (TouchedComponent :type Primitive%20Component%20Object%20Reference))
  (Rendering|SetRenderCustomDepth (Variables|Default|Getpayphone) true))

(event OnEndCursorOver(payphone)
  (params (TouchedComponent :type Primitive%20Component%20Object%20Reference))
  (Rendering|SetRenderCustomDepth (Variables|Default|Getpayphone) false))

(fn ConstructionScript)