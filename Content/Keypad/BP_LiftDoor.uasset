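; Lift door actor that slides two door panels open and shut, ending the game once it has fully opened.
; OpenLift and CloseLift each play a timeline that moves the right panel along local Y and mirrors the left around a fixed offset.
; When opening finishes, it calls FinishGame on the player's FirstPersonCharacter, then closes the doors after a delay; a failed cast skips both steps.
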(event Custom|OpenLift
  (bind _rightdoor (Variables|Default|GetRightDoor))
  (bind _leftdoor (Variables|Default|GetLeftDoor))
  (bind _relativelocation (Variables|/Script/Engine.SceneComponent|GetRelativeLocation _rightdoor))
  (bind _relativelocation_2 (Variables|/Script/Engine.SceneComponent|GetRelativeLocation _leftdoor))
  (bind _newtrack_0 (Timeline|Open PlayFromStart)
    (:Update
      (Transformation|SetRelativeLocation _rightdoor (Math|Vector|MakeVector (.x _relativelocation) _newtrack_0 (.z _relativelocation)) false false)
      (Transformation|SetRelativeLocation _leftdoor (Math|Vector|MakeVector (.x _relativelocation_2) (+ (* _newtrack_0 -1.0) 9e+01) (.z _relativelocation_2)) false false))
    (:Finished
      (bind _asfirst_person_character (Utilities|Casting|CastToFirstPersonCharacter (Game|GetPlayerCharacter 0)))
      (Default|FinishGame _asfirst_person_character)
      (Utilities|FlowControl|Delay 1e+01)
      (CallFunction|CloseLift))))

(event Custom|CloseLift
  (bind _rightdoor (Variables|Default|GetRightDoor))
  (bind _leftdoor (Variables|Default|GetLeftDoor))
  (bind _relativelocation (Variables|/Script/Engine.SceneComponent|GetRelativeLocation _rightdoor))
  (bind _relativelocation_2 (Variables|/Script/Engine.SceneComponent|GetRelativeLocation _leftdoor))
  (bind _newtrack_0 (Timeline|Timeline_0 PlayFromStart)
    (:Update
      (Transformation|SetRelativeLocation _rightdoor (Math|Vector|MakeVector (.x _relativelocation) _newtrack_0 (.z _relativelocation)) false false)
      (Transformation|SetRelativeLocation _leftdoor (Math|Vector|MakeVector (.x _relativelocation_2) (+ (* _newtrack_0 -1.0) 9e+01) (.z _relativelocation_2)) false false))))

(fn ConstructionScript)