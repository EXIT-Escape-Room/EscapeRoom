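; BP_KeyLockedDoor is a child door Blueprint that the player opens with a key.
; Overlapping OpenRange enables input if the first-person character has the door key, otherwise it prints a key-needed message.
; Clicking the mesh calls UseKey when the active inventory item is "Key".
; UseKey rechecks the key flag, then a timeline rotates the mesh's yaw and clears the flag.
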(event OnClicked(StaticMesh)
  (params (TouchedComponent :type Primitive%20Component%20Object%20Reference) (ButtonPressed :type Key%20Structure :default "None"))
  (bind _asfirst_person_character (Utilities|Casting|CastToFirstPersonCharacter (Game|GetPlayerCharacter 0)))
  (if (Utilities|Enum|Equal(Enum) (Utilities|GetActiveItem _asfirst_person_character) "Key")
    (CallFunction|UseKey)))

(event OnComponentBeginOverlap(OpenRange)
  (params (OverlappedComponent :type Primitive%20Component%20Object%20Reference) (OtherActor :type Actor%20Object%20Reference) (OtherComp :type Primitive%20Component%20Object%20Reference) (OtherBodyIndex :type Integer) (bFromSweep :type Boolean) (SweepResult :type Hit%20Result%20Structure%20%28by%20ref%29))
  (bind _asfirst_person_character (Utilities|Casting|CastToFirstPersonCharacter OtherActor))
  (if (Variables|/Game/FirstPersonBP/Blueprints/FirstPersonCharacter.FirstPersonCharacter_C|GetHasDoorKey _asfirst_person_character)
    (Input|EnableInput (Game|GetPlayerController 0))
    (else
      (Development|PrintString "Key needed"))))

(event Custom|UseKey
  (bind _asfirst_person_character (Utilities|Casting|CastToFirstPersonCharacter (Game|GetPlayerCharacter 0)))
  (if (Variables|/Game/FirstPersonBP/Blueprints/FirstPersonCharacter.FirstPersonCharacter_C|GetHasDoorKey _asfirst_person_character)
    (bind _newtrack_0 (Timeline|Timeline_0 PlayFromStart)
      (:Update
        (Transformation|SetRelativeRotation (Variables|Default|GetStaticMesh) (Math|Rotator|MakeRotator 0.0 0.0 _newtrack_0) false false)
        (Variables|/Game/FirstPersonBP/Blueprints/FirstPersonCharacter.FirstPersonCharacter_C|SetHasDoorKey _asfirst_person_character false)))))

(event EventBeginPlay
  (|CallParentFunction)
  (Variables|Default|SetHandledByChild true))

(event Collision|EventActorEndOverlap
  (params (OtherActor :type Actor%20Object%20Reference))
  (|CallParentFunction OtherActor))

(fn ConstructionScript
  (|CallParentFunction))