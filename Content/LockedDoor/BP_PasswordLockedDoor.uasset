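; Password-locked door, a child of a base door class, that swings open on a timeline once it is solved.
; Clicking the mesh toggles a WB_Numpad widget that targets this door, switching input mode as it appears or is removed.
; Input is enabled at BeginPlay, so physical digit, Backspace and Enter keys forward to the numpad.
; DoorOpening checks Solved before rotating the mesh's yaw; the OpenRange overlap events do nothing.
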(event OnComponentBeginOverlap(OpenRange)
  (params (OverlappedComponent :type Primitive%20Component%20Object%20Reference) (OtherActor :type Actor%20Object%20Reference) (OtherComp :type Primitive%20Component%20Object%20Reference) (OtherBodyIndex :type Integer) (bFromSweep :type Boolean) (SweepResult :type Hit%20Result%20Structure%20%28by%20ref%29)))

(event OnComponentEndOverlap(OpenRange)
  (params (OverlappedComponent :type Primitive%20Component%20Object%20Reference) (OtherActor :type Actor%20Object%20Reference) (OtherComp :type Primitive%20Component%20Object%20Reference) (OtherBodyIndex :type Integer)))

(event OnClicked(StaticMesh)
  (params (TouchedComponent :type Primitive%20Component%20Object%20Reference) (ButtonPressed :type Key%20Structure :default "None"))
  (bind _returnvalue (Game|GetPlayerController 0))
  (bind _returnvalue_2 (Game|GetPlayerController 0))
  (Utilities|FlowControl|FlipFlop
    (:A
      (bind _returnvalue_3 (UserInterface|CreateWidget "/Game/LockedDoor/WB_Numpad.WB_Numpad_C" 0 "" 0))
      (Variables|Default|SetNumpadWidget _returnvalue_3)
      (Variables|/Game/LockedDoor/WB_Numpad.WB_Numpad_C|SetTargetDoor _returnvalue_3 self)
      (UserInterface|Viewport|AddtoViewport _returnvalue_3 0)
      (Input|SetInputModeGameandUI _returnvalue_2 _returnvalue_3 "DoNotLock" true)
      (Variables|/Script/Engine.PlayerController|SetbShowMouseCursor _returnvalue_2 true))
    (:B
      (Viewport|RemoveAllWidgets)
      (Input|SetInputModeGameOnly _returnvalue)
      (Variables|/Script/Engine.PlayerController|SetbShowMouseCursor _returnvalue true))))

(event Custom|DoorOpening
  (if (Variables|Default|GetSolved)
    (bind _newtrack_0 (Timeline|DoorOpen Play)
      (:Update
        (Transformation|SetRelativeRotation (Variables|Default|GetStaticMesh) (Math|Rotator|MakeRotator 0.0 0.0 (* _newtrack_0 -1.0)) false false)))))

(event EventBeginPlay
  (|CallParentFunction)
  (Variables|Default|SetHandledByChild true)
  (Utilities|Casting|CastToFirstPersonCharacter (Game|GetPlayerCharacter 0))
  (Input|EnableInput (Game|GetPlayerController 0)))

(event Input|KeyboardEvents|1
  (params (Key :type Key%20Structure :default "None"))
  ;[1 1 1] Use keyboard events to type in numpad (allows for physical keyboard usage)
  (:Pressed
    (Default|Handle1 (Variables|Default|GetNumpadWidget))))

(event Input|KeyboardEvents|E
  (params (Key :type Key%20Structure :default "None")))

(event Input|KeyboardEvents|0
  (params (Key :type Key%20Structure :default "None"))
  ;[1 1 1] Use keyboard events to type in numpad (allows for physical keyboard usage)
  (:Pressed
    (Default|Handle0 (Variables|Default|GetNumpadWidget))))

(event Input|KeyboardEvents|Backspace
  (params (Key :type Key%20Structure :default "None"))
  ;[1 1 1] Use keyboard events to type in numpad (allows for physical keyboard usage)
  (:Pressed
    (Default|HandleBackspace (Variables|Default|GetNumpadWidget))))

(event Input|KeyboardEvents|Enter
  (params (Key :type Key%20Structure :default "None"))
  ;[1 1 1] Use keyboard events to type in numpad (allows for physical keyboard usage)
  (:Pressed
    (Default|HandleEnter (Variables|Default|GetNumpadWidget))))

(event Input|KeyboardEvents|2
  (params (Key :type Key%20Structure :default "None"))
  ;[1 1 1] Use keyboard events to type in numpad (allows for physical keyboard usage)
  (:Pressed
    (Default|Handle2 (Variables|Default|GetNumpadWidget))))

(event Input|KeyboardEvents|3
  (params (Key :type Key%20Structure :default "None"))
  ;[1 1 1] Use keyboard events to type in numpad (allows for physical keyboard usage)
  (:Pressed
    (Default|Handle3 (Variables|Default|GetNumpadWidget))))

(event Input|KeyboardEvents|4
  (params (Key :type Key%20Structure :default "None"))
  ;[1 1 1] Use keyboard events to type in numpad (allows for physical keyboard usage)
  (:Pressed
    (Default|Handle4 (Variables|Default|GetNumpadWidget))))

(event Input|KeyboardEvents|5
  (params (Key :type Key%20Structure :default "None"))
  ;[1 1 1] Use keyboard events to type in numpad (allows for physical keyboard usage)
  (:Pressed
    (Default|Handle5 (Variables|Default|GetNumpadWidget))))

(event Input|KeyboardEvents|6
  (params (Key :type Key%20Structure :default "None"))
  ;[1 1 1] Use keyboard events to type in numpad (allows for physical keyboard usage)
  (:Pressed
    (Default|Handle6 (Variables|Default|GetNumpadWidget))))

(event Input|KeyboardEvents|7
  (params (Key :type Key%20Structure :default "None"))
  ;[1 1 1] Use keyboard events to type in numpad (allows for physical keyboard usage)
  (:Pressed
    (Default|Handle7 (Variables|Default|GetNumpadWidget))))

(event Input|KeyboardEvents|8
  (params (Key :type Key%20Structure :default "None"))
  ;[1 1 1] Use keyboard events to type in numpad (allows for physical keyboard usage)
  (:Pressed
    (Default|Handle8 (Variables|Default|GetNumpadWidget))))

(event Input|KeyboardEvents|9
  (params (Key :type Key%20Structure :default "None"))
  ;[1 1 1] Use keyboard events to type in numpad (allows for physical keyboard usage)
  (:Pressed
    (Default|Handle9 (Variables|Default|GetNumpadWidget))))

(fn ConstructionScript
  (|CallParentFunction))