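; Locked chest puzzle actor that opens with the chest key and highlights through custom depth on cursor hover.
; If the ladder is placed, clicking teleports the player to an angled view, while pressing C teleports them away.
; Box overlap enables input, locks rotation and arms the puzzle.
; Clicking then checks key and active item, updates inventory and swings the lid via timeline, or briefly shows a hint dialog without the key.
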(event OnComponentBeginOverlap(Box)
  (params (OverlappedComponent :type Primitive%20Component%20Object%20Reference) (OtherActor :type Actor%20Object%20Reference) (OtherComp :type Primitive%20Component%20Object%20Reference) (OtherBodyIndex :type Integer) (bFromSweep :type Boolean) (SweepResult :type Hit%20Result%20Structure%20%28by%20ref%29))
  (bind _asfirst_person_character (Utilities|Casting|CastToFirstPersonCharacter OtherActor))
  (Input|EnableInput (Game|GetPlayerController 0))
  (Variables|/Game/FirstPersonBP/Blueprints/FirstPersonCharacter.FirstPersonCharacter_C|SetCanRotate _asfirst_person_character false)
  (Variables|Default|SetattemptingPuzzle true))

(event OnComponentEndOverlap(Box)
  (params (OverlappedComponent :type Primitive%20Component%20Object%20Reference) (OtherActor :type Actor%20Object%20Reference) (OtherComp :type Primitive%20Component%20Object%20Reference) (OtherBodyIndex :type Integer))
  (bind _asfirst_person_character (Utilities|Casting|CastToFirstPersonCharacter OtherActor))
  (Input|DisableInput (Game|GetPlayerController 0))
  (Variables|/Game/FirstPersonBP/Blueprints/FirstPersonCharacter.FirstPersonCharacter_C|SetCanRotate _asfirst_person_character true)
  (Variables|Default|SetattemptingPuzzle false))

(event MouseInput|EventActorBeginCursorOver
  (Rendering|SetRenderCustomDepth (Variables|Default|GetChest) true))

(event MouseInput|EventActorEndCursorOver
  (Rendering|SetRenderCustomDepth (Variables|Default|GetChest) false))

(event MouseInput|EventActorOnClicked
  (params (ButtonPressed :type Key%20Structure :default "None"))
  (bind _chest (Variables|Default|GetChest))
  (bind _returnvalue (Transformation|GetWorldLocation _chest))
  (if (and (Variables|Default|GetattemptingPuzzle) (not (Variables|Default|Getsolved)))
    (if (Variables|/Game/FirstPersonBP/Blueprints/FirstPersonCharacter.FirstPersonCharacter_C|GetHasChestKey (stale OnComponentBeginOverlap(Box) _asfirst_person_character))
      (if (Utilities|Enum|Equal(Enum) (Variables|/Game/FirstPersonBP/Blueprints/FirstPersonCharacter.FirstPersonCharacter_C|GetActiveItem (stale OnComponentBeginOverlap(Box) _asfirst_person_character)) (Variables|Default|GetActiveItem))
        (Default|RemovefromInventoryWidget (Variables|/Game/FirstPersonBP/Blueprints/Inventory/BPC_Inventory.BPC_Inventory_C|GetInventoryWidget (Variables|/Game/FirstPersonBP/Blueprints/FirstPersonCharacter.FirstPersonCharacter_C|GetBPC_Inventory (stale OnComponentBeginOverlap(Box) _asfirst_person_character))) (Utilities|Struct|MakeS_ItemInfo "Key"))
        (Variables|/Game/FirstPersonBP/Blueprints/FirstPersonCharacter.FirstPersonCharacter_C|SetActiveItem (stale OnComponentBeginOverlap(Box) _asfirst_person_character) "Key")
        (Variables|Default|Setsolved true)
        (bind _chest_track (Timeline|OpenChest PlayFromStart)
          (:Update
            (Transformation|SetRelativeRotation (Variables|Default|GetLid) (Math|Rotator|MakeRotator 0.0 (Math|Float|Lerp (Variables|Default|GetClosedAngle) (Variables|Default|GetOpenAngle) _chest_track) 0.0) false false)
            (Variables|Default|SetIsOpen true))))
      (else
        (Variables|Default|GetIsValid
          (:then)
          (:else
            (bind _returnvalue_2 (UserInterface|CreateWidget "/Game/FirstPersonBP/Feedback/WB_CharacterDialog.WB_CharacterDialog_C" 0 "I must find something to unlock this chest. "))
            (bind _output_get (Variables|Default|SetIsValid _returnvalue_2))
            (UserInterface|Viewport|AddtoViewport _output_get 0)
            (Utilities|FlowControl|Delay 5.0)
            (Widget|RemovefromParent _output_get)))))
    (else
      (bind _asfirst_person_character (Utilities|Casting|CastToFirstPersonCharacter (Game|GetPlayerCharacter 0)))
      (if (Variables|/Game/FirstPersonBP/Blueprints/FirstPersonCharacter.FirstPersonCharacter_C|GetLadderPlaced _asfirst_person_character)
        (CallFunction|MoveCharacter (+ (.x _returnvalue) -1e+02) (.y _returnvalue) 4e+02 -3e+01)))))

(event Input|KeyboardEvents|C
  (params (Key :type Key%20Structure :default "None"))
  (:Pressed
    (CallFunction|MoveCharacter 6e+02 6e+02 1.5e+02 0.0)))

(fn ConstructionScript)

(fn MoveCharacter
  (params (TargetX :type Float%20%28single-precision%29) (TargetY :type Float%20%28single-precision%29) (TargetZ :type Float%20%28single-precision%29) (TargetAngle :type Float%20%28single-precision%29))
  (bind _asfirst_person_character (Utilities|Casting|CastToFirstPersonCharacter (Game|GetPlayerCharacter 0)))
  (Transformation|SetWorldLocation (Variables|/Script/Engine.Actor|GetRootComponent _asfirst_person_character) (Math|Vector|MakeVector TargetX TargetY TargetZ) false false)
  (Transformation|SetWorldRotation (Variables|/Game/FirstPersonBP/Blueprints/FirstPersonCharacter.FirstPersonCharacter_C|GetFirstPersonCamera _asfirst_person_character) (Math|Rotator|MakeRotator 0.0 TargetAngle (- (.yaw (Transformation|GetWorldRotation (Variables|Default|GetArrow))) 1.8e+02)) false false))