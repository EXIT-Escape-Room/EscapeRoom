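; Clickable empty picture frame that launches the jigsaw puzzle and displays its picture once the puzzle is solved.
; On click, player character flags and the active item decide between opening the jigsaw widget, which disables character rotation, or showing a timed hint dialog.
; Tick polls the solved flag to unhide the initially hidden picture.
; Cursor hover toggles custom depth on the mesh.
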(event OnClicked(StaticMesh)
  (params (TouchedComponent :type Primitive%20Component%20Object%20Reference) (ButtonPressed :type Key%20Structure :default "None"))
  (bind _asfirst_person_character (Utilities|Casting|CastToFirstPersonCharacter (Game|GetPlayerCharacter 0)))
  (if (not (Variables|/Game/FirstPersonBP/Blueprints/FirstPersonCharacter.FirstPersonCharacter_C|GetJigsawPuzzleSolved _asfirst_person_character))
    (if (Variables|/Game/FirstPersonBP/Blueprints/FirstPersonCharacter.FirstPersonCharacter_C|GetPictureSeen _asfirst_person_character)
      (if (Variables|/Game/FirstPersonBP/Blueprints/FirstPersonCharacter.FirstPersonCharacter_C|GetHasJigsawPieces _asfirst_person_character)
        (bind _activeitem (Utilities|GetActiveItem))
        (if (Utilities|Enum|Equal(Enum) _activeitem (Variables|Default|GetActiveItem))
          (Variables|Default|GetJigsawWidget
            (:then)
            (:else
              (bind _returnvalue (UserInterface|CreateWidget "/Game/JigsawPuzzle/WB_JigsawWidget.WB_JigsawWidget_C" (Game|GetPlayerController 0)))
              (bind _output_get (Variables|Default|SetJigsawWidget _returnvalue))
              (UserInterface|Viewport|AddtoViewport _output_get 0)
              (bind _asfirst_person_character_2 (Utilities|Casting|CastToFirstPersonCharacter (Game|GetPlayerCharacter 0)))
              (Variables|/Game/FirstPersonBP/Blueprints/FirstPersonCharacter.FirstPersonCharacter_C|SetCanRotate _asfirst_person_character_2 false))))
        (else
          (Variables|Default|GetIsValid
            (:then)
            (:else
              (bind _returnvalue_2 (UserInterface|CreateWidget "/Game/FirstPersonBP/Feedback/WB_CharacterDialog.WB_CharacterDialog_C" 0 "Empty frame, weird... I might have to place a painting here."))
              (Variables|Default|SetIsValid _returnvalue_2)
              (UserInterface|Viewport|AddtoViewport _returnvalue_2 0)
              (Utilities|FlowControl|Delay 3.0)
              (Widget|RemovefromParent _returnvalue_2)
              (Variables|Default|SetIsValid 0)))))
      (else
        (Variables|Default|GetIsValid1
          (:then)
          (:else
            (bind _returnvalue_3 (UserInterface|CreateWidget "/Game/FirstPersonBP/Feedback/WB_CharacterDialog.WB_CharacterDialog_C" 0 "I'm not  sure how to place the pieces here. Maybe I'll find something helpful in the room."))
            (Variables|Default|SetIsValid1 _returnvalue_3)
            (UserInterface|Viewport|AddtoViewport _returnvalue_3 0)
            (Utilities|FlowControl|Delay 3.0)
            (Widget|RemovefromParent _returnvalue_3)
            (Variables|Default|SetIsValid1 0)))))))

(event EventBeginPlay
  (Development|SetHiddeninGame (Variables|Default|GetPicture) true false))

(event Collision|EventActorBeginOverlap
  (params (OtherActor :type Actor%20Object%20Reference)))

(event EventTick
  (params (DeltaSeconds :type Float%20%28single-precision%29))
  (bind _asfirst_person_character (Utilities|Casting|CastToFirstPersonCharacter (Game|GetPlayerCharacter 0)))
  (if (Variables|/Game/FirstPersonBP/Blueprints/FirstPersonCharacter.FirstPersonCharacter_C|GetJigsawPuzzleSolved _asfirst_person_character)
    (Development|SetHiddeninGame (Variables|Default|GetPicture) false false)))

(event MouseInput|EventActorBeginCursorOver
  (Rendering|SetRenderCustomDepth (Variables|Default|GetStaticMesh) true))

(event MouseInput|EventActorEndCursorOver
  (Rendering|SetRenderCustomDepth (Variables|Default|GetStaticMesh) false))

(fn ConstructionScript)